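; BP_GunProjectile is a gun projectile that sticks to what it hits and can then be picked up with a motion controller.
; Its first Box hit on anything other than a DestructibleActor welds it to the hit component and destroys ProjectileMovement.
; Pickup, called by BP_MotionController, works only after that hit, disabling physics and attaching to the given component; Drop enables physics and detaches.
; A delayed self-destroy is present but unwired.
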(event OnComponentBeginOverlap(StaticMesh)
  (params (OverlappedComponent :type Primitive%20Component%20Object%20Reference) (OtherActor :type Actor%20Object%20Reference) (OtherComp :type Primitive%20Component%20Object%20Reference) (OtherBodyIndex :type Integer) (bFromSweep :type Boolean) (SweepResult :type Hit%20Result%20Structure%20%28by%20ref%29)))

(event OnComponentHit(Box)
  (params (HitComponent :type Primitive%20Component%20Object%20Reference) (OtherActor :type Actor%20Object%20Reference) (OtherComp :type Primitive%20Component%20Object%20Reference) (NormalImpulse :type Vector :default "0, 0, 0") (Hit :type Hit%20Result%20Structure%20%28by%20ref%29))
  (Utilities|Casting|CastToDestructibleActor OtherActor
    (:CastFailed
      (Utilities|FlowControl|DoOnce false
        (:Completed
          (Variables|Default|SetHasHit true)
          (Transformation|AttachComponentToComponent OtherComp "None" "KeepWorld" "KeepWorld" "KeepWorld" true)
          (Components|DestroyComponent (Variables|Default|GetProjectileMovement)))))))

(event EventBeginPlay)

(event EventTick
  (params (DeltaSeconds :type Float%20%28single-precision%29)))

(event EventPickup
  (params (AttachTo :type Scene%20Component%20Object%20Reference))
  (if (Variables|Default|GetHasHit)
    (Physics|SetSimulatePhysics (Variables|Default|GetBox) false)
    (Transformation|AttachComponentToComponent (VehicleSound|GetRootComponent) AttachTo "None" "KeepWorld" "KeepWorld" "KeepWorld" false)))

(event EventDrop
  (Physics|SetSimulatePhysics (Variables|Default|GetBox) true)
  (Transformation|DetachFromActor "KeepWorld" "KeepWorld" "KeepWorld"))

(fn ConstructionScript)