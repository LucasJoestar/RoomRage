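; Gravity gun Blueprint that pulls physics objects while the E key is held.
; Each tick while attracting, it line-traces for PhysicsBody objects from AttractPoint, with the end built from that point's world location rotated by the first found CameraActor's rotation and scaled by AttractRange.
; Hits receive a force back along the trace at the impact point, scaled by hit distance divided by AttractForce, with debug drawing and prints.
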(event EventTick
  (params (DeltaSeconds :type Float%20%28single-precision%29))
  (bind _attract_point (Variables|Default|GetAttract%20Point))
  (bind _returnvalue (Transformation|GetWorldLocation _attract_point))
  (if (Variables|Default|GetIsAttracting)
    (bind (_outhit _returnvalue_2) (Collision|LineTraceForObjects _returnvalue (* (Math|Vector|RotateVector _returnvalue (Transformation|GetActorRotation (Variables|Default|GetCamera))) (Variables|Default|GetAttractRange)) (Utilities|Array|MakeArray "ObjectTypeQuery4") false 0 "ForOneFrame"))
    (if _returnvalue_2
      (Class|PrimitiveComponent|AddForceatLocation (.hitcomponent _outhit) (* (- (.tracestart _outhit) (.traceend _outhit)) (/ (.distance _outhit) (Variables|Default|GetAttractForce))) (.impactpoint _outhit) "None")
      (Development|PrintString "Hit"))))

(event EventBeginPlay
  (bind _outactors (Actor|GetAllActorsOfClass "/Script/Engine.CameraActor"))
  (Variables|Default|SetCamera (Utilities|Array|Get(acopy) _outactors)))

(event Input|KeyboardEvents|E
  (params (Key :type Key%20Structure))
  (:Pressed
    (Variables|Default|SetIsAttracting true)
    (Development|PrintString "Attracting"))
  (:Released
    (Variables|Default|SetIsAttracting false)
    (Development|PrintString "NO attracting")))

(fn ConstructionScript)