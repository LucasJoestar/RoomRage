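; Gravity gun actor that pulls physics objects in front of it, holds them and launches them.
; While attraction is on (Shoot event or left mouse), Tick line-traces forward from AttractPoint and applies a distance-normalized force with angular damping.
; Close objects attach to AttractPoint with physics off; releasing re-enables physics.
; Expulse (right mouse) launches the current object with a forward impulse; CCD is enabled on targets.
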(event Custom|Expulse
  ;[1 1 1] Expulse attracting object
  (if (Utilities|IsValid (Variables|Default|GetObjectAttracting))
    (Physics|SetSimulatePhysics (Variables|Default|GetObjectAttracting) true)
    (Class|PrimitiveComponent|SetAllPhysicsLinearVelocity (Variables|Default|GetObjectAttracting) "0, 0, 0" false)
    (Physics|AddImpulse (Variables|Default|GetObjectAttracting) (* (* (Transformation|GetActorForwardVector) (Variables|Default|GetExpulseForce)) 100) "None" false)
    (Variables|Default|SetObjectAttracting 0)
    (Variables|Default|SetIsAttracting false)))

(event EventShoot
  (params (Pressed :type Boolean))
  ;[1 1 1] Enable / disable attraction when pressing / relasing E key
  (if Pressed
    (Variables|Default|SetIsAttracting true)
    (else
      (Variables|Default|SetIsAttracting false)
      (if (Utilities|IsValid (Variables|Default|GetObjectAttracting))
        (Physics|SetSimulatePhysics (Variables|Default|GetObjectAttracting) true))
      (Variables|Default|SetObjectAttracting 0))))

(event EventTick
  (params (DeltaSeconds :type Float%20%28single-precision%29))
  (bind _attract_point (Variables|Default|GetAttract%20Point))
  (bind _returnvalue (Transformation|GetWorldLocation _attract_point))
  ;[1 1 1] Attract objects in front of the Player
  (if (Variables|Default|GetIsAttracting)
    (bind (_outhit _returnvalue_2) (Collision|LineTraceForObjects _returnvalue (+ _returnvalue (* (Transformation|GetActorForwardVector) (Variables|Default|GetAttractRange))) (Utilities|Array|MakeArray "ObjectTypeQuery4") false 0 "ForOneFrame"))
    (if _returnvalue_2
      (if (== (Variables|Default|GetObjectAttracting) (.hitcomponent _outhit))
        _
        (else
          (if (Utilities|IsValid (Variables|Default|GetObjectAttracting))
            (Physics|SetSimulatePhysics (Variables|Default|GetObjectAttracting) true))
          (Class|PrimitiveComponent|SetUseCCD (.hitcomponent _outhit) true "None")
          (Variables|Default|SetObjectAttracting (.hitcomponent _outhit))))
      (if (<= (.distance _outhit) 1e+02)
        (Transformation|AttachComponentToComponent (Components|GetOwner (Variables|Default|GetObjectAttracting)) (Variables|Default|GetAttract%20Point) "None" "KeepWorld" "KeepWorld" "KeepWorld" false)
        (Physics|SetSimulatePhysics (Variables|Default|GetObjectAttracting) false)
        (else
          (Class|PrimitiveComponent|SetAllPhysicsAngularVelocityinDegrees (Variables|Default|GetObjectAttracting) (* (Physics|GetPhysicsAngularVelocityinDegrees (Variables|Default|GetObjectAttracting) "None") 0.93) false)
          (Class|PrimitiveComponent|AddForceatLocation (Variables|Default|GetObjectAttracting) (* (* (- (.tracestart _outhit) (.location _outhit)) (/ (Variables|Default|GetAttractForce) (.distance _outhit))) 100) (.impactpoint _outhit) "None")))
      (elif (Utilities|IsValid (Variables|Default|GetObjectAttracting))
        (Physics|SetSimulatePhysics (Variables|Default|GetObjectAttracting) true)
        (Variables|Default|SetObjectAttracting 0)))))

(event EventBeginPlay
  ;[1 1 1] Get player camera at Start
  (if (not (Class|HeadMountedDisplayFunctionLibrary|IsHeadMountedDisplayEnabled))
    (bind _outactors (Actor|GetAllActorsOfClass "/Script/Engine.PlayerCameraManager"))
    (Variables|Default|SetCamera (Utilities|Array|Get(acopy) _outactors))))

(event Input|MouseEvents|LeftMouseButton
  (params (Key :type Key%20Structure))
  ;[1 1 1] Enable / disable attraction when pressing / relasing E key
  (:Pressed
    (Variables|Default|SetIsAttracting true))
  (:Released
    (Variables|Default|SetIsAttracting false)
    (if (Utilities|IsValid (Variables|Default|GetObjectAttracting))
      (Physics|SetSimulatePhysics (Variables|Default|GetObjectAttracting) true))
    (Variables|Default|SetObjectAttracting 0)))

(event Input|MouseEvents|RightMouseButton
  (params (Key :type Key%20Structure))
  ;[1 1 1] Expulse attracting object
  (:Pressed
    (if (Utilities|IsValid (Variables|Default|GetObjectAttracting))
      (Physics|SetSimulatePhysics (Variables|Default|GetObjectAttracting) true)
      (Class|PrimitiveComponent|SetAllPhysicsLinearVelocity (Variables|Default|GetObjectAttracting) "0, 0, 0" false)
      (Physics|AddImpulse (Variables|Default|GetObjectAttracting) (* (* (Transformation|GetActorForwardVector) (Variables|Default|GetExpulseForce)) 100) "None" false)
      (Variables|Default|SetObjectAttracting 0)
      (Variables|Default|SetIsAttracting false))))

(fn ConstructionScript)