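; Gravity gun that pulls physics objects in front of it toward an attract point, then drops or launches them.
; While attracting, Tick sphere-traces forward, updates the tracked list, and applies distance-normalized force with angular damping.
; Objects within close range attach to the point with physics disabled.
; Left mouse or the Shoot event toggles attraction on press and release; right mouse or Expulse launches tracked objects forward by impulse.
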(event Custom|Expulse
  ;[1 1 1] Expulse attracting object
  (for _array_element (Variables|Default|GetObjectAttracting)
    (Physics|SetSimulatePhysics _array_element true)
    (Class|PrimitiveComponent|SetAllPhysicsLinearVelocity _array_element "0, 0, 0" false)
    (Physics|AddImpulse _array_element (* (* (Transformation|GetActorForwardVector) (Variables|Default|GetExpulseForce)) 1000) "None" false))
  (Utilities|Array|Clear (Variables|Default|GetObjectAttracting))
  (Variables|Default|SetIsAttracting false))

(event Custom|ResetAttractingObjects
  (bind _objectattracting (Variables|Default|GetObjectAttracting))
  ;[1 1 1] Clear Attracting Objects and enable their physics
  (for _array_element _objectattracting
    (Physics|SetSimulatePhysics _array_element true))
  (Utilities|Array|Clear _objectattracting))

(event EventShoot
  (params (Pressed :type Boolean))
  ;[1 1 1] Enable / disable attraction when pressing / relasing E key
  (if Pressed
    (Variables|Default|SetIsAttracting true)
    (else
      (CallFunction|ResetAttractingObjects)
      (Variables|Default|SetIsAttracting false))))

(event EventTick
  (params (DeltaSeconds :type Float%20%28single-precision%29))
  (bind _attract_point (Variables|Default|GetAttract%20Point))
  (bind _returnvalue (Transformation|GetWorldLocation _attract_point))
  ;[1 1 1] Attract objects in front of the Player
  (if (Variables|Default|GetIsAttracting)
    (bind _outhits (Collision|MultiSphereTraceForObjects _returnvalue (+ _returnvalue (* (Transformation|GetActorForwardVector) (Variables|Default|GetAttractRange))) 0.0 (Utilities|Array|MakeArray "ObjectTypeQuery4") false 0 "None"))
    (Utilities|FlowControl|Sequence
      (:then_0
        (for _array_element (Variables|Default|GetObjectAttracting)
          (bind _array_element_2 (Utilities|Array|ForEachLoopwithBreak _outhits :!label _label)
            (:LoopBody
              (if (== _array_element (.hitcomponent _array_element_2))
                (Variables|Default|Setcontains true)
                (goto _label Break)))
            (:Completed
              (if (Variables|Default|Getcontains)
                (Variables|Default|Setcontains false)
                (else
                  (Physics|SetSimulatePhysics _array_element true)
                  (Utilities|Array|RemoveItem (Variables|Default|GetObjectAttracting) _array_element)))))))
      (:then_1
        (for _array_element_3 _outhits
          (if (Utilities|Array|ContainsItem (Variables|Default|GetObjectAttracting) (.hitcomponent _array_element_3))
            _
            (else
              (Utilities|Array|Add (Variables|Default|GetObjectAttracting) (.hitcomponent _array_element_3))
              (Physics|SetSimulatePhysics (.hitcomponent _array_element_3) true)
              (Class|PrimitiveComponent|SetUseCCD (.hitcomponent _array_element_3) true "None")))
          (if (<= (.distance _array_element_3) 1e+02)
            (Transformation|AttachComponentToComponent (Components|GetOwner (.hitcomponent _array_element_3)) (Variables|Default|GetAttract%20Point) "None" "KeepWorld" "KeepWorld" "KeepWorld" false)
            (Physics|SetSimulatePhysics (.hitcomponent _array_element_3) false)
            (else
              (Class|PrimitiveComponent|SetAllPhysicsAngularVelocityinDegrees (.hitcomponent _array_element_3) (* (Physics|GetPhysicsAngularVelocityinDegrees (.hitcomponent _array_element_3) "None") 0.93) false)
              (Class|PrimitiveComponent|AddForceatLocation (.hitcomponent _array_element_3) (* (* (- (.tracestart _array_element_3) (.location _array_element_3)) (/ (Variables|Default|GetAttractForce) (.distance _array_element_3))) 1000) (.impactpoint _array_element_3) "None"))))))))

(event EventBeginPlay
  ;[1 1 1] Get player camera at Start
  (if (not (Class|HeadMountedDisplayFunctionLibrary|IsHeadMountedDisplayEnabled))
    (bind _outactors (Actor|GetAllActorsOfClass "/Script/Engine.PlayerCameraManager"))
    (Variables|Default|SetCamera (Utilities|Array|Get(acopy) _outactors))))

(event Input|MouseEvents|LeftMouseButton
  (params (Key :type Key%20Structure))
  ;[1 1 1] Enable / disable attraction when pressing / relasing E key
  (:Pressed
    (Variables|Default|SetIsAttracting true))
  (:Released
    (CallFunction|ResetAttractingObjects)
    (Variables|Default|SetIsAttracting false)))

(event Input|MouseEvents|RightMouseButton
  (params (Key :type Key%20Structure))
  ;[1 1 1] Expulse attracting object
  (:Pressed
    (for _array_element (Variables|Default|GetObjectAttracting)
      (Physics|SetSimulatePhysics _array_element true)
      (Class|PrimitiveComponent|SetAllPhysicsLinearVelocity _array_element "0, 0, 0" false)
      (Physics|AddImpulse _array_element (* (* (Transformation|GetActorForwardVector) (Variables|Default|GetExpulseForce)) 1000) "None" false))
    (Utilities|Array|Clear (Variables|Default|GetObjectAttracting))
    (Variables|Default|SetIsAttracting false)))

(fn ConstructionScript)